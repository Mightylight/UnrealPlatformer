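; BP_TempPlatform is a temporary platform that vanishes after the player character touches it, then returns.
; An overlap from BP_ThirdPersonCharacter starts a two-second delay, after which the root's visibility toggles with propagation to children and the ShapePlane mesh is cleared.
; Two seconds later it toggles visibility again and restores the Floor_400x400 mesh.
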(event Collision|EventActorBeginOverlap
  (params (OtherActor :type Actor%20Object%20Reference))
  (Utilities|Casting|CastToBP_ThirdPersonCharacter OtherActor)
  (Utilities|FlowControl|Delay 2.0)
  (Rendering|ToggleVisibility (Variables|Default|GetDefaultSceneRoot) true)
  (Components|StaticMesh|SetStaticMesh (Variables|Default|GetShape_Plane) 0)
  (Utilities|FlowControl|Delay 2.0)
  (Rendering|ToggleVisibility (Variables|Default|GetDefaultSceneRoot) true)
  (Components|StaticMesh|SetStaticMesh (Variables|Default|GetShape_Plane) "/Game/StarterContent/Architecture/Floor_400x400.Floor_400x400"))

(fn ConstructionScript)