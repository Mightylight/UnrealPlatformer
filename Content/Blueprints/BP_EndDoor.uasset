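; BP_EndDoor is a locked door that the player opens and closes with E when carrying the key.
; Overlapping it as BP_ThirdPersonCharacter caches the player and enables input on the actor, with no end-overlap to disable it.
; A FlipFlop alternately plays and reverses a Timeline that drives the door mesh's yaw, and ShapeCube is destroyed when the Timeline finishes.
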(event Collision|EventActorBeginOverlap
  (params (OtherActor :type Actor%20Object%20Reference))
  (bind _asbp_third_person_character (Utilities|Casting|CastToBP_ThirdPersonCharacter OtherActor))
  (Variables|Default|SetPlayer _asbp_third_person_character)
  (Input|EnableInput (Game|GetPlayerController 0)))

(event Input|KeyboardEvents|E
  (params (Key :type Key%20Structure :default "None"))
  (:Pressed
    (if (Variables|/Game/ThirdPerson/Blueprints/BP_ThirdPersonCharacter.BP_ThirdPersonCharacter_C|GethasKey (Variables|Default|GetPlayer))
      (Utilities|FlowControl|FlipFlop
        (:A
          (bind _doorrotation (Timeline|Timeline Play)
            (:Update
              (Transformation|SetRelativeRotation (Variables|Default|GetSM_Door) (Math|Rotator|MakeRotator 0.0 0.0 _doorrotation) false false))
            (:Finished
              (Components|DestroyComponent (Variables|Default|GetShape_Cube)))))
        (:B
          (Timeline|Timeline Reverse))))))

(fn ConstructionScript)