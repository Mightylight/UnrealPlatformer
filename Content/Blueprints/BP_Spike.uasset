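; BP_Spike is a hazard actor that damages the third-person player character while they overlap it.
; On begin overlap it stores the character, applies one hit of damage immediately and starts a looping timer that repeats the damage at a fixed interval.
; On end overlap by that character it clears the stored timer handle to stop the damage.
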(event Custom|DamagePlayer
  (Game|Damage|ApplyDamage (Variables|Default|GetPlayer) 1.0 0 0))

(event Collision|EventActorBeginOverlap
  (params (OtherActor :type Actor%20Object%20Reference))
  (bind _asbp_third_person_character (Utilities|Casting|CastToBP_ThirdPersonCharacter OtherActor))
  (bind _output_get (Variables|Default|SetPlayer _asbp_third_person_character))
  (Game|Damage|ApplyDamage _output_get 1.0 0 0)
  (bind _returnvalue (Utilities|Time|SetTimerbyEvent (delegate Custom|DamagePlayer) 2.0 true))
  (Variables|Default|SetNewVar _returnvalue))

(event Collision|EventActorEndOverlap
  (params (OtherActor :type Actor%20Object%20Reference))
  (Utilities|Casting|CastToBP_ThirdPersonCharacter OtherActor)
  (Utilities|Time|ClearandInvalidateTimerbyHandle (Variables|Default|GetNewVar)))

(fn ConstructionScript)